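; BP_MapPawn is a level selection pawn Blueprint with no active logic, as BeginPlay and the construction script are empty.
; An unconnected, never-run graph finds a BP_MapSpline and plays a Timeline at a rate of 1 / NewRate.
; That draft logic lerps the Timeline track over the spline length to set the pawn's world location and rotation along the spline.
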(event `self.ReceiveBeginPlay`)

(event `Key|Left`
  (params (Key :type "Key Structure")))

(event `Key|Right`
  (params (Key :type "Key Structure")))

(fn `UserConstructionScript`)