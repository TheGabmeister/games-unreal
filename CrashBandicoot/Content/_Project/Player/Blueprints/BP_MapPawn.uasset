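; BP_MapPawn is a map pawn that travels automatically along a spline path when play begins.
; BeginPlay finds the BP_MapSpline actor in the level and starts a Timeline with play rate set to the inverse of NewRate.
; Each update maps the Timeline track to a distance along the spline and sets the pawn's world location and rotation to match that point.
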(event `self.ReceiveBeginPlay`
  (bind _spline (`/Game/_Project/LevelSelection/BP_MapSpline.Spline` (`self.Spline`)))
  (bind _returnvalue (`GameplayStatics.GetActorOfClass` "/Game/_Project/LevelSelection/BP_MapSpline.BP_MapSpline_C"))
  (set `self.Spline` _returnvalue)
  (`TimelineComponent.SetPlayRate` (`self.Timeline`) (/ 1.0 (`self.New Rate`)))
  (bind (_direction _track) (`Timeline|Timeline`)
    (:`Update`
      (bind _returnvalue_2 (`KismetMathLibrary.Lerp` 0.0 (`SplineComponent.GetSplineLength` (`/Game/_Project/LevelSelection/BP_MapSpline.Spline` (`self.Spline`))) _track))
      (`self.K2_SetActorTransform` (`KismetMathLibrary.MakeTransform` (`SplineComponent.GetLocationAtDistanceAlongSpline` _spline _returnvalue_2 "World") (`SplineComponent.GetRotationAtDistanceAlongSpline` _spline _returnvalue_2 "World"))))))

(fn `UserConstructionScript`)