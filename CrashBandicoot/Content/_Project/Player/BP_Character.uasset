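; BP_Character is the player character, with a follow camera that moves along a level spline.
; On BeginPlay it finds the BP_Spline actor and stores its spline component.
; Each tick it finds the spline point closest to the character and eases the camera toward it with interpolation, giving a smoothed rail-style camera.
; Only the camera's location is updated here, not its rotation.
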(event `self.ReceiveBeginPlay`
  (bind _returnvalue (`GameplayStatics.GetActorOfClass` "/Game/_Project/LevelSelection/BP_Spline.BP_Spline_C"))
  (set `self.Spline` (`SplineActor.SplineComp` _returnvalue)))

(event `self.ReceiveTick`
  (params (DeltaSeconds :type "Float (single-precision)"))
  ; Move Camera
  (`SceneComponent.K2_SetWorldLocation` (`self.FollowCamera`) (`KismetMathLibrary.VInterpTo` (`SceneComponent.K2_GetComponentLocation` (`self.FollowCamera`)) (`SplineComponent.FindLocationClosestToWorldLocation` (`self.Spline`) (`self.K2_GetActorLocation`) "World") (`GameplayStatics.GetWorldDeltaSeconds`) 2.0) false false))

(fn `UserConstructionScript`)